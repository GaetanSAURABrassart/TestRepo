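; A physics-driven six-sided die for a board game that is thrown and reports the face it lands on.
; Throw teleports the die to a throw point, randomizes its rotation, adds a random angular impulse and starts a looping poll timer.
; Once velocity is near zero, it compares three arrow components and their inverses against a world-up arrow to cache the top face, then clears the timer.
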(event `self.Throw`
  (set `self.CachedResult` 0)
  ;[0 0 0] Teleport to Throw point
  (`SceneComponent.K2_SetWorldLocation` (`self.Die`) (`SceneComponent.K2_GetComponentLocation` (`self.ThrowPoint`)) true true)
  ;[0 0 0] Random rotation
  (`SceneComponent.K2_SetWorldRotation` (`self.Die`) (`KismetMathLibrary.RandomRotator` true) false false)
  ;[0 0 0] Add impulse to Die
  (`PrimitiveComponent.AddAngularImpulseInDegrees` (`self.Die`) (* (`self.ImpulseSpeed`) (`KismetMathLibrary.RandomUnitVector`)) "None" true)
  (bind _returnvalue (`KismetSystemLibrary.K2_SetTimerDelegate` (delegate `WaitingResult`) 0.5 true true)))

(event `WaitingResult`
  (bind (_bisequal _bisinvert) (`self.ComparePolarVector` (`self.GetWorldUpVector`) (`SceneComponent.GetForwardVector` (`self.RightArrow`))))
  (bind (_bisequal_2 _bisinvert_2) (`self.ComparePolarVector` (`self.GetWorldUpVector`) (`SceneComponent.GetForwardVector` (`self.UpArrow`))))
  (bind (_bisequal_3 _bisinvert_3) (`self.ComparePolarVector` (`self.GetWorldUpVector`) (`SceneComponent.GetForwardVector` (`self.ForwardArrow`))))
  (if (`KismetMathLibrary.NearlyEqual_FloatFloat` (`self.GetDieVelocity`) 0.0 (`self.AngularTolerance`))
    (if _bisequal_3
      (set `self.CachedResult` 6)
      (`KismetSystemLibrary.K2_ClearAndInvalidateTimerHandle` (stale `self.Throw` _returnvalue) :!label _label)
      (elif _bisinvert_3
        (set `self.CachedResult` 1)
        (goto _label)
        (elif _bisequal_2
          (set `self.CachedResult` 5)
          (goto _label)
          (elif _bisinvert_2
            (set `self.CachedResult` 2)
            (goto _label)
            (elif _bisequal
              (set `self.CachedResult` 4)
              (goto _label)
              (elif _bisinvert
                (set `self.CachedResult` 3)
                (goto _label)
                (else
                  (set `self.CachedResult` 0))))))))))

(fn `ComparePolarVector`
  (params (VectorA :type "Vector Structure") (VectorB :type "Vector Structure"))
  (returns (bIsEqual :type Boolean) (bIsInvert :type Boolean))
  (bind _angulartolerance (`self.AngularTolerance`))
  (return (== VectorA VectorB :`ErrorTolerance` _angulartolerance) (== VectorA (* VectorB -1.0) :`ErrorTolerance` _angulartolerance)))

(fn `GetDieVelocity`
  (returns (ReturnValue :type "Float (double-precision)"))
  (return (`KismetMathLibrary.VSize` (`SceneComponent.GetComponentVelocity` (`self.Die`)))))

(fn `GetWorldUpVector`
  (returns (WorldUpVector :type "Vector Structure"))
  (return (`SceneComponent.GetForwardVector` (`self.WorldUp`))))

(fn `UserConstructionScript`
  (`parent.UserConstructionScript`))