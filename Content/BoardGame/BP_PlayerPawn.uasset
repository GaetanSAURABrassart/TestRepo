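; Player pawn for a board game that throws a dice and moves its game piece along the board's cells.
; The throw input rolls the Dice, then a looping timer polls until the result is above zero.
; The result is added to the piece's position, bounded by the board's cell count, and the piece is placed on that cell.
; Construction and BeginPlay also snap the piece to its current cell.
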(event `self.ReceiveBeginPlay`
  (bind _cell (`/Game/BoardGame/Board/BP_Board.GetBoardCellByPosition` (`self.Board`) (`/Game/BoardGame/BP_PawnActor.Position` (`self.Pawn`))))
  (`/Game/BoardGame/BP_PawnActor.PlaceOnCell` (`self.Pawn`) _cell))

(event `EnhancedInput|/Game/BoardGame/Input/Action/IA_Throw`
  (params (ActionValue :type Boolean) (ElapsedSeconds :type "Float (double-precision)") (TriggeredSeconds :type "Float (double-precision)") (InputAction :type "InputAction Object Reference" :default "/Game/BoardGame/Input/Action/IA_Throw.IA_Throw"))
  (:`Started`
    (`self.DiceThrow`)))

(event `DiceThrow`
  ;[0 0 0] Throw Dice
  (`/Game/BoardGame/Dice/BP_Die.Throw` (`self.Dice`))
  (bind _returnvalue (`KismetSystemLibrary.K2_SetTimerDelegate` (delegate `WaitingResult`) 0.5 true true)))

(event `WaitingResult`
  (if (> (`/Game/BoardGame/Dice/BP_Die.GetResult` (`self.Dice`)) 0)
    (`self.AfterWaitingResult`)
    (`KismetSystemLibrary.K2_ClearAndInvalidateTimerHandle` (stale `DiceThrow` _returnvalue))))

(event `AfterWaitingResult`
  (bind _result (`/Game/BoardGame/Dice/BP_Die.GetResult` (`self.Dice`)))
  (`KismetSystemLibrary.PrintString` (`KismetStringLibrary.Conv_IntToString` _result))
  ;[0 0 0] Add Result to Position
  (`/Game/BoardGame/BP_PawnActor.AddResultToPosition` (`self.Pawn`) _result (`/Game/BoardGame/Board/BP_Board.GetCellsLength` (`self.Board`)))
  ;[0 0 0] Get Board Cell by Position
  (bind _cell (`/Game/BoardGame/Board/BP_Board.GetBoardCellByPosition` (`self.Board`) (`/Game/BoardGame/BP_PawnActor.Position` (`self.Pawn`))))
  ;[0 0 0] Place Pawn On Cell
  (`/Game/BoardGame/BP_PawnActor.PlaceOnCell` (`self.Pawn`) _cell))

(fn `UserConstructionScript`
  (bind _cell (`/Game/BoardGame/Board/BP_Board.GetBoardCellByPosition` (`self.Board`) (`/Game/BoardGame/BP_PawnActor.Position` (`self.Pawn`))))
  (`/Game/BoardGame/BP_PawnActor.PlaceOnCell` (`self.Pawn`) _cell))